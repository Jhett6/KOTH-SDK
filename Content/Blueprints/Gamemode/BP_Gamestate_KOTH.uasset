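; Game state Blueprint for the King of the Hill (KOTH) game mode.
; Its one custom function, GetMSV, takes a controller and returns the MSVs entry for that controller's team, or an empty result if the controller is invalid.
; BeginPlay and the construction script only call their parents, and Tick is disabled.
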(event EventBeginPlay
  (|CallParentFunction))

(event EventTick
  (params (DeltaSeconds :type Float%20%28single-precision%29))
  (|CallParentFunction DeltaSeconds) ; This node is disabled and will not be called.\nDrag off pins to build functionality.
)

(fn ConstructionScript
  (|CallParentFunction))

(fn GetMSV
  (params (Controller :type BP%20Player%20Controller%20KOTH%20Object%20Reference))
  (Utilities|IsValid Controller
    (:Is%20Valid
      (return (Utilities|Array|Get(acopy) (Variables|Default|GetMSVs) (Class|SQPlayerController|GetTeam Controller))))
    (:Is%20Not%20Valid
      (return 0))))