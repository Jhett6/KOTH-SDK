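; Vehicle spawner actor for the KOTH game mode, tied to a team.
; On BeginPlay, the server fetches the KOTH ruleset and, if valid, adds itself with its team to the ruleset's SpawnersForTeams collection.
; CanSpawnHere runs a box overlap for SQVehicle actors in its Box volume, returning whether the spot is clear along with any blocking vehicles.
; The spawner itself contains no spawn logic.
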(event EventBeginPlay
  (Networking|SwitchHasAuthority
    (:Authority
      (bind _outruleset (CallFunction|GetKOTHRuleset))
      (bind _output_get (Variables|Default|SetRuleset _outruleset))
      (Utilities|IsValid _output_get
        (:Is%20Valid
          (Utilities|Map|Add (Variables|/KingOfTheHill/Blueprints/BP_Ruleset_KOTH.BP_Ruleset_KOTH_C|GetSpawnersForTeams _output_get) self (Variables|Default|GetTeam)))))))

(event Collision|EventActorBeginOverlap
  (params (OtherActor :type Actor%20Object%20Reference)))

(event EventTick
  (params (DeltaSeconds :type Float%20%28single-precision%29)))

(fn ConstructionScript)

(fn CanSpawnHere
  (bind _box (Variables|Default|GetBox))
  (bind (_outactors _returnvalue) (Collision|BoxOverlapActors (Transformation|GetWorldLocation _box) (Components|Box|GetScaledBoxExtent _box) (Utilities|Array|MakeArray "ObjectTypeQuery5") "/Script/Squad.SQVehicle" :!class /Script/Engine.KismetSystemLibrary))
  (return _outactors (not _returnvalue)))