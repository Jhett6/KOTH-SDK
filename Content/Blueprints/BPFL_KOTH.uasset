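; Blueprint function library of helpers for the KOTH game mode.
; GetKOTHRuleset fetches the BP_Ruleset_KOTH ruleset from the Squad game mode and is marked server-only.
; TeamIDToEnum maps a numeric ID to neutral, team one or team two.
; SetupMSV registers a vehicle in the KOTH game state's MSVs array, using the slot that matches the vehicle's team.
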(fn GetKOTHRuleset
  (bind ___worldcontext (LocalVariables|Get__WorldContext))
  (bind _return_value (CallFunction|GetSquadGameMode ___worldcontext))
  ;[1 1 1] Get Ruleset (Server Only)
  (Utilities|IsValid _return_value
    (:Is%20Valid
      (bind _outruleset (Class|SQGameMode|TryGetRulesetOfClass _return_value "/KingOfTheHill/Blueprints/BP_Ruleset_KOTH.BP_Ruleset_KOTH_C"))
      (return _outruleset))))

(fn TeamIDtoEnum
  (params (ID :type Integer))
  (switch int ID
    (:0
      (return "Team_Neutral"))
    (:1
      (return "Team_One"))
    (:2
      (return "Team_Two"))))

(fn SetupMSV
  (params (Vehicle :type SQ%20Vehicle%20Object%20Reference))
  (Utilities|IsValid Vehicle
    (:Is%20Valid
      (bind _asbp_gamestate_koth (Utilities|Casting|CastToBP_Gamestate_KOTH (CallFunction|GetSquadGameState Vehicle)))
      (LocalVariables|SetAs%20BP%20Gamestate%20KOTH _asbp_gamestate_koth)
      (switch Utilities|FlowControl|Switch|SwitchonESQTeam (Variables|/Script/Squad.SQPawn|GetTeam Vehicle)
        (:Team_Neutral
          (Utilities|Array|SetArrayElem (Variables|/KingOfTheHill/Blueprints/Gamemode/BP_Gamestate_KOTH.BP_Gamestate_KOTH_C|GetMSVs (LocalVariables|GetAs%20BP%20Gamestate%20KOTH)) 0 Vehicle))
        (:Team_One
          (Utilities|Array|SetArrayElem (Variables|/KingOfTheHill/Blueprints/Gamemode/BP_Gamestate_KOTH.BP_Gamestate_KOTH_C|GetMSVs (LocalVariables|GetAs%20BP%20Gamestate%20KOTH)) 1 Vehicle))
        (:Team_Two
          (Utilities|Array|SetArrayElem (Variables|/KingOfTheHill/Blueprints/Gamemode/BP_Gamestate_KOTH.BP_Gamestate_KOTH_C|GetMSVs (LocalVariables|GetAs%20BP%20Gamestate%20KOTH)) 2 Vehicle))))))