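; BP_KOTH_Tower is a King of the Hill capture zone tower whose map icon shows which team has the most occupants.
; UIUpdate tallies Occupants per team, then finds the highest count.
; Each team matching that count adds its green, blue or red colour, and the sum is divided by the number of matches, so ties show a blended tint.
; An empty tower shows a white icon.
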(fn ConstructionScript)

(fn UIUpdate
  (bind _l_mixedelementcount (LocalVariables|GetL_MixedElementCount))
  (bind _returnvalue (Math|Conversions|ToFloat(Integer) _l_mixedelementcount))
  (if (> (Utilities|Array|Length (Variables|Default|GetOccupants)) 0)
    (for _array_element (Variables|Default|GetOccupants)
      (if true
        (Utilities|Array|SetArrayElem (LocalVariables|GetL_SoldierCountPerTeam) (Class|SQSoldier|GetTeam _array_element) (+ (Utilities|Array|Get(acopy) (LocalVariables|GetL_SoldierCountPerTeam) (Class|SQSoldier|GetTeam _array_element)) 1) true)))
    (LocalVariables|SetL_MaxPlayer (.MaxValue (Math|Integer|MaxOfIntArray (LocalVariables|GetL_SoldierCountPerTeam))))
    (for (_array_element_2 _array_index) (LocalVariables|GetL_SoldierCountPerTeam)
      (Math|Integer|CompareInt _array_element_2 (LocalVariables|GetL_MaxPlayer)
        (:==
          (LocalVariables|SetColour (+ (LocalVariables|GetColour) (Utilities|Select :Index _array_index :Option%200 "(R=0.000000,G=1.000000,B=0.000000,A=1.000000)" :Option%201 "(R=0.000000,G=0.000000,B=1.000000,A=1.000000)" :Option%202 "(R=1.000000,G=0.000000,B=0.000000,A=1.000000)")))
          (Math|Integer|IncrementInt (LocalVariables|GetL_MixedElementCount)))))
    (Variables|/Script/Squad.SQMapItemComponent|SetTint (Variables|Default|GetMapIcon) (/ (LocalVariables|GetColour) (Utilities|Struct|MakeLinearColor _returnvalue _returnvalue _returnvalue _returnvalue)))
    (else
      (Variables|/Script/Squad.SQMapItemComponent|SetTint (Variables|Default|GetMapIcon) "(R=1.000000,G=1.000000,B=1.000000,A=1.000000)"))))