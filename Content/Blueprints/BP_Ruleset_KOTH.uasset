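; BP_Ruleset_KOTH is a ruleset Blueprint, named for the KOTH mode, that acts as an effectively unlimited rearm source.
; Any pawn may rearm, each weapon decides through its own CanRearm, and ammo consumption always succeeds against a huge constant supply.
; Rearm type is MainOrEnvironment, feedback strings are empty, and ammo-update binding is stubbed to return false because no stock is tracked.
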(fn ConstructionScript)

(fn BindEventtoAmmoUpdated
  (params (Delegate :type Delegate%20%28by%20ref%29))
  (return false))

(fn CanRearmPawn
  (params (Rearmer :type Pawn%20Object%20Reference))
  (return true))

(fn CanRearmWeapon
  (params (Weapon :type SQ%20Equipable%20Item%20Object%20Reference))
  (return (Class|SQEquipableItem|CanRearm Weapon)))

(fn ConsumeAmmo
  (params (AmmoRequired :type Float%20%28single-precision%29))
  (return true))

(fn GetAmmo
  (return 1e+05))

(fn GetRearmNoAmmoString
  (return ""))

(fn GetRearmSuccessString
  (return ""))

(fn GetRearmType
  (return "MainOrEnvironment"))

(fn UnbindEventtoAmmoUpdated
  (params (Delegate :type Delegate%20%28by%20ref%29))
  (return false))